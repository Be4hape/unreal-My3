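; BPc_Soldier is a player-controlled soldier pawn that handles movement, turning and fire input.
; Axis inputs move it along its forward vector and add controller yaw to turn it.
; Action inputs for move, rotate left, rotate right and fire only set boolean state flags on press and clear them on release.
; Nothing in this Blueprint reads those flags, and BeginPlay, Tick, overlap and the construction script are empty.
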(event EventBeginPlay)

(event Collision|EventActorBeginOverlap
  (params (OtherActor :type Actor%20Object%20Reference)))

(event EventTick
  (params (DeltaSeconds :type Float%20%28single-precision%29)))

(event Input|ActionEvents|InputActionPlayer_fire
  (params (Key :type Key%20Structure :default "None"))
  (:Pressed
    (Variables|Default|SetisFire true))
  (:Released
    (Variables|Default|SetisFire false)))

(event Input|ActionEvents|InputActionPlayer_Move
  (params (Key :type Key%20Structure :default "None"))
  (:Pressed
    (Variables|Default|SetisMove true))
  (:Released
    (Variables|Default|SetisMove false)))

(event Input|ActionEvents|InputActionPlayer_RotR
  (params (Key :type Key%20Structure :default "None"))
  (:Pressed
    (Variables|Default|SetisRotR true))
  (:Released
    (Variables|Default|SetisRotR false)))

(event Input|ActionEvents|InputActionPlayer_RotL
  (params (Key :type Key%20Structure :default "None"))
  (:Pressed
    (Variables|Default|SetisRotL true))
  (:Released
    (Variables|Default|SetisRotL false)))

(event Input|AxisEvents|InputAxisPlayer_Move
  (params (AxisValue :type Float%20%28single-precision%29))
  (Pawn|Input|AddMovementInput (Transformation|GetActorForwardVector) AxisValue false))

(event Input|AxisEvents|InputAxisPlayer_Rotate
  (params (AxisValue :type Float%20%28single-precision%29))
  (Pawn|Input|AddControllerYawInput AxisValue))

(fn ConstructionScript)